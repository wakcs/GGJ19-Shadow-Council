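; BP_CollectableSpawner is an actor that keeps spawning random collectable types inside its Zone box, randomized on the Y and Z axes only.
; On BeginPlay it divides the base delay range by the game mode's player count times difficulty, so higher values spawn faster.
; Tick feeds a random Delay that paces spawning, and each new actor joins CurrentCollectables, whose oldest entry is destroyed once the count exceeds MaxCollectables.
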(event `self.ReceiveBeginPlay`
  (`self.Setmin and max spawn for coins`))

(event `self.ReceiveTick`
  (params (DeltaSeconds :type "Float (single-precision)"))
  (bind _currentcollectables (`self.CurrentCollectables`))
  (bind _output (`|GetArrayItem` _currentcollectables))
  (`KismetSystemLibrary.Delay` (`KismetMathLibrary.RandomFloatInRange` (`self.minDelay`) (`self.maxDelay`)))
  (if (> (`KismetArrayLibrary.Array_Length` _currentcollectables) (`self.maxCollectables`))
    (`/Engine/EditorBlueprintResources/StandardMacros.IsValid` _output
      (:`Is Valid`
        (`self.K2_DestroyActor` _output))
      (:`Is Not Valid`
        _))
    (`KismetArrayLibrary.Array_Remove` _currentcollectables))
  (`self.SpawnCollectableInZone`))

(fn `Setmin and max spawn for coins`
  (bind _asgm_base_game_mode (cast `/Game/Core/GM_BaseGameMode` (`GameplayStatics.GetGameMode`)))
  (bind _returnvalue (* (`KismetMathLibrary.Conv_IntToDouble` (`/Game/Core/GM_BaseGameMode.PlayerCount` _asgm_base_game_mode)) (`/Game/Core/GM_BaseGameMode.Difficulty` _asgm_base_game_mode)))
  (set `self.minDelay` (/ (`self.baseminDelay`) _returnvalue))
  (set `self.maxDelay` (/ (`self.basemaxDelay`) _returnvalue)))

(fn `SpawnCollectableInZone`
  (bind _collectabletypes (`self.CollectableTypes`))
  (bind (_returnvalue_x _returnvalue_y _returnvalue_z) (`KismetMathLibrary.BreakVector` (`BoxComponent.GetScaledBoxExtent` (`self.Zone`))))
  (bind _returnvalue (`|SpawnActorFromClass` (`|GetArrayItem` _collectabletypes (`KismetMathLibrary.RandomInteger` (`KismetArrayLibrary.Array_Length` _collectabletypes))) (`KismetMathLibrary.MakeTransform` (+ (`self.K2_GetActorLocation`) (`KismetMathLibrary.MakeVector` 0.0 (`KismetMathLibrary.RandomFloatInRange` (* _returnvalue_y -1.0) _returnvalue_y) (`KismetMathLibrary.RandomFloatInRange` (* _returnvalue_z -1.0) _returnvalue_z)))) "AdjustIfPossibleButDontSpawnIfColliding" "OverrideRootScale" null null))
  (`KismetArrayLibrary.Array_Add` (`self.CurrentCollectables`) _returnvalue))

(fn `UserConstructionScript`)