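; Base house actor that acts as a balance platform, tilting under the weight of players inside it.
; HouseCollider overlaps track each player's BPC_Mass component.
; While any are tracked, Tick sums torque-like forces from mass, gravity and offset from PivotPoint, plus a decaying ExternalForce.
; Each Tick rolls BasePlane by the last computed force, scaled by BalanceSensitivity and clamped to RotationMax; UpdateMassObjects is an empty stub.
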(event `self.ReceiveTick`
  (params (DeltaSeconds :type "Float (single-precision)"))
  (`|ExecutionSequence`
    (:`then_0`
      (`self.UpdateMassObjects`))
    (:`then_1`
      (if (not (== (`KismetArrayLibrary.Array_Length` (`self.MassObjects`)) 0))
        (`self.CalculateForces`)
        (`self.UpdateGravityVector`)))
    (:`then_2`
      (`self.RotatePlatform`))))

(event `self.HouseCollider.OnComponentBeginOverlap`
  (params (OverlappedComponent :type "PrimitiveComponent Object Reference") (OtherActor :type "Actor Object Reference") (OtherComp :type "PrimitiveComponent Object Reference") (OtherBodyIndex :type Integer) (bFromSweep :type Boolean) (SweepResult :type "HitResult Structure (by ref)"))
  (bind _asbp_base_player (cast `/Game/Core/BP_BasePlayer` OtherActor))
  (`KismetArrayLibrary.Array_AddUnique` (`self.MassObjects`) (`/Game/Core/BP_BasePlayer.BPC_Mass` _asbp_base_player)))

(event `self.HouseCollider.OnComponentEndOverlap`
  (params (OverlappedComponent :type "PrimitiveComponent Object Reference") (OtherActor :type "Actor Object Reference") (OtherComp :type "PrimitiveComponent Object Reference") (OtherBodyIndex :type Integer))
  (bind _asbp_base_player (cast `/Game/Core/BP_BasePlayer` OtherActor))
  (`KismetArrayLibrary.Array_RemoveItem` (`self.MassObjects`) (`/Game/Core/BP_BasePlayer.BPC_Mass` _asbp_base_player)))

(fn `CalculateForces`
  (`|ExecutionSequence`
    (:`then_0`
      ;[1 1 1] Reset Final Force
      (set `self.FinalForce` (0.0 0.0 0.0)))
    (:`then_1`
      (for _array_element (`self.MassObjects`)
        (bind _individualforce (`self.CalculateIndividualForce` _array_element))
        ;[1 1 1] Append Forces
        (bind _output_get (set `self.FinalForce` (+ (`self.FinalForce`) (`KismetMathLibrary.MakeVector` 0.0 (.y _individualforce) (.x _individualforce)) (`self.External Force`))))))
    (:`then_2`
      (set `self.External Force` (* (`self.External Force`) 0.5)))))

(fn `CalculateIndividualForce`
  (params (`Mass Component` :type "/Game/Core/BPC_Mass Object Reference"))
  (returns (IndividualForce :type "Vector Structure") (ReturnValue :type "Vector Structure"))
  (locals (Mass :type "Float (double-precision)") (OwnerLocation :type "Vector Structure"))
  (`|ExecutionSequence`
    (:`then_0`
      (set `local.Mass` (`/Game/Core/BPC_Mass.Mass` `Mass Component`))
      (set `local.OwnerLocation` (`self.K2_GetActorLocation` (`ActorComponent.GetOwner` `Mass Component`))))
    (:`then_1`
      (return (* (`self.CalculateDistance` (`local.OwnerLocation`) (`SceneComponent.K2_GetComponentLocation` (`self.PivotPoint`))) (* (`self.BaseGravity`) (`local.Mass`))) (0.0 0.0 0.0)))))

(fn `RotatePlatform`
  (bind (_returnvalue_roll _returnvalue_pitch _returnvalue_yaw) (`KismetMathLibrary.BreakRotator` (`self.K2_GetActorRotation`)))
  (bind (_returnvalue_roll_2 _returnvalue_pitch_2 _returnvalue_yaw_2) (`KismetMathLibrary.BreakRotator` (`self.K2_GetActorRotation`)))
  (bind _rotationmax (`self.RotationMax`))
  (bind (_finalforce_x _finalforce_y) (`KismetMathLibrary.BreakVector` (`self.FinalForce`)))
  (bind _returnvalue_roll_3 (`KismetMathLibrary.BreakRotator` (`SceneComponent.K2_GetComponentRotation` (`self.BasePlane`))))
  (`SceneComponent.K2_AddRelativeRotation` (`self.BasePlane`) (`KismetMathLibrary.MakeRotator` (* (`KismetMathLibrary.FClamp` (`KismetMathLibrary.NormalizeToRange` _finalforce_y 0.0 (`self.BalanceSensitivity`)) -1.0) -1.0)) false false)
  ;[1 1 1] Checkin If Roation is going over the Rotation Amount
  (`|ExecutionSequence`
    (:`then_0`
      (if (>= _returnvalue_roll_3 _rotationmax)
        ;[1 1 1] Set Rotation When Going Over RotationMax
        (`SceneComponent.K2_SetWorldRotation` (`self.BasePlane`) (`KismetMathLibrary.MakeRotator` (`self.RotationMax`) _returnvalue_pitch _returnvalue_yaw) false false)))
    (:`then_1`
      (if (<= _returnvalue_roll_3 (* _rotationmax -1.0))
        (`SceneComponent.K2_SetWorldRotation` (`self.BasePlane`) (`KismetMathLibrary.MakeRotator` (* (`self.RotationMax`) -1.0) _returnvalue_pitch_2 _returnvalue_yaw_2) false false)))))

(fn `UpdateGravityVector`
  (returns (UpdatedGravityVector :type "Vector Structure"))
  (set `self.GravityVector` (0.0 0.0 -1.0))
  (return (0.0 0.0 0.0)))

(fn `UpdateMassObjects`)

(fn `UserConstructionScript`)