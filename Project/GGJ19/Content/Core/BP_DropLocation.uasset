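; BP_DropLocation is a drop point that spawns an actor at a set height and lowers it toward the plane.
; Tick polls SpawnNext behind a delay, moves the spawned actor down at constant speed, and sets SpawnNext when a downward trace finds the plane close beneath it.
; A second trace keeps the Warning widget above the plane.
; DropComplete activates the BP_MassActor's mass component and removes the drop point; DropFail destroys both.
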(event `self.ReceiveTick`
  (params (DeltaSeconds :type "Float (single-precision)"))
  (bind (_returnvalue_x _returnvalue_y) (`KismetMathLibrary.BreakVector` (`self.K2_GetActorLocation`)))
  (bind (_returnvalue_x_2 _returnvalue_y_2) (`KismetMathLibrary.BreakVector` (`self.K2_GetActorLocation`)))
  (bind (_returnvalue_x_3 _returnvalue_y_3) (`KismetMathLibrary.BreakVector` (`self.K2_GetActorLocation`)))
  (bind _returnvalue (`self.K2_GetActorLocation`))
  (bind _warning (`self.Warning`))
  (bind _spawned_actor_ref (`self.Spawned Actor Ref`))
  (bind _spawned_actor_ref_2 (`self.Spawned Actor Ref`))
  (bind _spawned_actor_ref_3 (`self.Spawned Actor Ref`))
  (bind (_returnvalue_x_4 _returnvalue_y_4 _returnvalue_z) (`KismetMathLibrary.BreakVector` (`self.K2_GetActorLocation` _spawned_actor_ref_3)))
  (bind _returnvalue_2 (`self.K2_GetActorLocation` _spawned_actor_ref_2))
  (`|ExecutionSequence`
    (:`then_0`
      (`KismetSystemLibrary.Delay` 10.0)
      (if (`self.SpawnNext`)
        (set `self.SpawnNext` false)
        (bind _returnvalue_3 (`|SpawnActorFromClass` (`self.Spawned Actor Class`) (`KismetMathLibrary.MakeTransform` (`KismetMathLibrary.MakeVector` _returnvalue_x _returnvalue_y (`self.Spawn Height`))) "Undefined" "OverrideRootScale" null null null))
        (set `self.Spawned Actor Ref` _returnvalue_3)
        (set `/Game/Core/BP_MassActor.DropLocation` self _returnvalue_3)))
    (:`then_1`
      (`|ExecutionSequence`
        (:`then_0`
          (`/Engine/EditorBlueprintResources/StandardMacros.IsValid` _spawned_actor_ref_3
            (:`Is Valid`
              ;[1 1 1] Move object down and stop it when near plane
              (if (> _returnvalue_z (`self.EndHeight`))
                (`/Engine/EditorBlueprintResources/StandardMacros.IsValid` _spawned_actor_ref
                  (:`Is Valid`
                    (`self.K2_SetActorLocation` _spawned_actor_ref (`KismetMathLibrary.VInterpTo_Constant` (`self.K2_GetActorLocation` (`self.Spawned Actor Ref`)) (`KismetMathLibrary.MakeVector` _returnvalue_x_2 _returnvalue_y_2 (`self.EndHeight`)) (`GameplayStatics.GetWorldDeltaSeconds`) (`self.Drop Speed`)) false false)
                    (`/Engine/EditorBlueprintResources/StandardMacros.IsValid` _spawned_actor_ref_2
                      (:`Is Valid`
                        (bind (_outhit _returnvalue_4) (`KismetSystemLibrary.LineTraceSingleForObjects` _returnvalue_2 (`KismetMathLibrary.MakeVector` (.x _returnvalue_2) (.y _returnvalue_2) (`self.EndHeight`)) (`|MakeArray` "ObjectTypeQuery8" :!type "EObjectTypeQuery Enum")))
                        (if _returnvalue_4
                          (if (<= (`.Distance` (`GameplayStatics.BreakHitResult` _outhit)) 2.0)
                            (set `self.SpawnNext` true)))))))
                (else
                  (set `self.SpawnNext` false))))))
        (:`then_1`
          ;[1 1 1] Set warning widget on plane
          (`/Engine/EditorBlueprintResources/StandardMacros.IsValid` (`self.Warning`)
            (:`Is Valid`
              (bind (_outhit_2 _returnvalue_5) (`KismetSystemLibrary.LineTraceSingleForObjects` _returnvalue (`KismetMathLibrary.MakeVector` (.x _returnvalue) (.y _returnvalue) (`self.EndHeight`)) (`|MakeArray` "ObjectTypeQuery8" :!type "EObjectTypeQuery Enum")))
              (if _returnvalue_5
                (`SceneComponent.K2_SetWorldLocation` _warning (`KismetMathLibrary.MakeVector` (.x (`.Location` (`GameplayStatics.BreakHitResult` _outhit_2))) (.y (`.Location` (`GameplayStatics.BreakHitResult` _outhit_2))) (+ (.z (`.Location` (`GameplayStatics.BreakHitResult` _outhit_2))) 50.0)) false true)
                (else
                  (`SceneComponent.K2_SetWorldLocation` _warning (`KismetMathLibrary.MakeVector` _returnvalue_x_3 _returnvalue_y_3 (`self.EndHeight`)) false true))))))))))

(fn `DropComplete`
  (bind _asbp_mass_actor (cast `/Game/Core/BP_MassActor` (`self.Spawned Actor Ref`)))
  (set `/Game/Core/BPC_Mass.Active` true (`/Game/Core/BP_MassActor.BPC_Mass` _asbp_mass_actor))
  (`self.K2_DestroyActor`))

(fn `DropFail`
  (`self.K2_DestroyActor` (`self.Spawned Actor Ref`))
  (`self.K2_DestroyActor`))

(fn `UserConstructionScript`)