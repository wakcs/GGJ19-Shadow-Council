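; BP_BasePlayer is a base player character Blueprint providing simple movement helpers and a camera shake test.
; Helper functions turn input X into movement along the actor's right vector and positive Y into a jump.
; A velocity check within an acceptance radius reports whether the player is standing still.
; The ShakeTest input plays a world camera shake at the main camera and prints a debug string.
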(event `InputAction|ShakeTest`
  (params (Key :type "Key Structure"))
  (:`Pressed`
    (`GameplayStatics.PlayWorldCameraShake` "/Game/Effects/BestCameraShake.BestCameraShake_C" (`SceneComponent.GetSocketLocation` (`self.MainCamera`) "None"))
    (`KismetSystemLibrary.PrintString` "U nerd")))

(fn `IsPlayerStandingStill`
  (params (AcceptanceRadius :type "Float (double-precision)"))
  (returns (IsStandingStill :type Boolean))
  (return (== (`MovementComponent.Velocity` (`self.CharacterMovement`)) (0.0 0.0 0.0) :`ErrorTolerance` AcceptanceRadius)))

(fn `PlayerMoveRight`
  (params (InptuScale :type "Vector2D Structure"))
  (`self.AddMovementInput` (`self.GetActorRightVector`) InptuScale_X))

(fn `PlayerMoveUp`
  (params (InptuScale :type "Vector2D Structure"))
  (if (> InptuScale_Y 0.0)
    (`self.Jump`)))

(fn `UserConstructionScript`)