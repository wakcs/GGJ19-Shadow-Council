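; BP_Ladder is a climbable ladder actor that tells players when they are in reach of it.
; Top and Bottom trigger volumes set the overlapping BP_BasePlayer's CloseLadder to this ladder and clear it on exit.
; The trigger entered also sets GoingUpLadder, true at the bottom and false at the top, while the climbing itself is not handled here.
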(event `self.Top.OnComponentBeginOverlap`
  (params (OverlappedComponent :type "PrimitiveComponent Object Reference") (OtherActor :type "Actor Object Reference") (OtherComp :type "PrimitiveComponent Object Reference") (OtherBodyIndex :type Integer) (bFromSweep :type Boolean) (SweepResult :type "HitResult Structure (by ref)"))
  (bind _asbp_base_player (cast `/Game/Core/BP_BasePlayer` OtherActor))
  (set `/Game/Core/BP_BasePlayer.CloseLadder` self _asbp_base_player)
  (set `/Game/Core/BP_BasePlayer.GoingUpLadder` false _asbp_base_player))

(event `self.Top.OnComponentEndOverlap`
  (params (OverlappedComponent :type "PrimitiveComponent Object Reference") (OtherActor :type "Actor Object Reference") (OtherComp :type "PrimitiveComponent Object Reference") (OtherBodyIndex :type Integer))
  (bind _asbp_base_player (cast `/Game/Core/BP_BasePlayer` OtherActor))
  (set `/Game/Core/BP_BasePlayer.CloseLadder` null _asbp_base_player))

(event `self.Bottom.OnComponentBeginOverlap`
  (params (OverlappedComponent :type "PrimitiveComponent Object Reference") (OtherActor :type "Actor Object Reference") (OtherComp :type "PrimitiveComponent Object Reference") (OtherBodyIndex :type Integer) (bFromSweep :type Boolean) (SweepResult :type "HitResult Structure (by ref)"))
  (bind _asbp_base_player (cast `/Game/Core/BP_BasePlayer` OtherActor))
  (set `/Game/Core/BP_BasePlayer.CloseLadder` self _asbp_base_player)
  (set `/Game/Core/BP_BasePlayer.GoingUpLadder` true _asbp_base_player))

(event `self.Bottom.OnComponentEndOverlap`
  (params (OverlappedComponent :type "PrimitiveComponent Object Reference") (OtherActor :type "Actor Object Reference") (OtherComp :type "PrimitiveComponent Object Reference") (OtherBodyIndex :type Integer))
  (bind _asbp_base_player (cast `/Game/Core/BP_BasePlayer` OtherActor))
  (set `/Game/Core/BP_BasePlayer.CloseLadder` null _asbp_base_player))

(fn `UserConstructionScript`)