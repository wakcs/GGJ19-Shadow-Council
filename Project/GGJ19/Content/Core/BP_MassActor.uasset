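; Mass object that lands on a BP_BaseHouse and adds its mass component until it is pushed or tipped off.
; On overlap it attaches, flips to suit the relative roll, registers, and plays explosion effects.
; PushoverBox hands itself to the player; Pushover counts pushes, shaking the mesh until tolerance.
; Tick maxes that count past a roll threshold; at tolerance it unregisters, detaches and launches the physics-enabled box.
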(event `Shake`
  (set `self.InitialRelativeLocation` (`SceneComponent.RelativeLocation` (`self.StaticMesh`)))
  (bind (_direction _newtrack_1) (`Timeline|ShakeT` :!via `PlayFromStart`)
    (:`Update`
      (`SceneComponent.K2_SetRelativeLocation` (`self.StaticMesh`) (+ _newtrack_1 (`self.InitialRelativeLocation`)) false false))))

(event `self.Box.OnComponentBeginOverlap`
  (params (OverlappedComponent :type "PrimitiveComponent Object Reference") (OtherActor :type "Actor Object Reference") (OtherComp :type "PrimitiveComponent Object Reference") (OtherBodyIndex :type Integer) (bFromSweep :type Boolean) (SweepResult :type "HitResult Structure (by ref)"))
  (bind _returnvalue_roll (`KismetMathLibrary.BreakRotator` (`self.K2_GetActorRotation`)))
  (bind _asbp_base_house (cast `/Game/Core/BP_BaseHouse` OtherActor))
  (if (not (>= (`self.CurrentPushover`) (`self.PushoverTolerance`)))
    (`/Engine/EditorBlueprintResources/StandardMacros.DoOnce` false
      (:`Completed`
        (set `/Game/Core/BP_DropLocation.Spawned Actor Ref` null (`self.DropLocation`))
        (bind _returnvalue_roll_2 (`KismetMathLibrary.BreakRotator` (`self.K2_GetActorRotation` _asbp_base_house)))
        (if (<= (`KismetMathLibrary.Abs` (- _returnvalue_roll_2 _returnvalue_roll)) 90.0)
          (`self.K2_AttachToComponent` OtherComp "None" "KeepWorld" "SnapToTarget" "KeepRelative" :!label _label)
          (else
            (`|ExecutionSequence`
              (:`then_0`
                (goto _label))
              (:`then_1`
                (`self.K2_AddActorLocalRotation` (struct :`Roll` 180.0))))))
        (`self.K2_AddActorLocalRotation` (struct :`Yaw` 180.0))
        (bind _outactors (`GameplayStatics.GetAllActorsOfClass` "/Game/Core/BP_BaseHouse.BP_BaseHouse_C"))
        (`KismetArrayLibrary.Array_AddUnique` (`/Game/Core/BP_BaseHouse.MassObjects` (`|GetArrayItem` _outactors)) (`self.BPC_Mass`))
        (`GameplayStatics.SpawnEmitterAtLocation` "/Game/Particle/P_Explosion.P_Explosion" (`self.K2_GetActorLocation`))
        (`GameplayStatics.PlaySound2D` (`self.SoundFile`) 1.0 1.0 0.0 null null)))))

(event `self.Pushover Box.OnComponentBeginOverlap`
  (params (OverlappedComponent :type "PrimitiveComponent Object Reference") (OtherActor :type "Actor Object Reference") (OtherComp :type "PrimitiveComponent Object Reference") (OtherBodyIndex :type Integer) (bFromSweep :type Boolean) (SweepResult :type "HitResult Structure (by ref)"))
  (bind _asbp_base_player (cast `/Game/Core/BP_BasePlayer` OtherActor))
  (set `/Game/Core/BP_BasePlayer.MassActor` self _asbp_base_player))

(event `self.Pushover Box.OnComponentEndOverlap`
  (params (OverlappedComponent :type "PrimitiveComponent Object Reference") (OtherActor :type "Actor Object Reference") (OtherComp :type "PrimitiveComponent Object Reference") (OtherBodyIndex :type Integer))
  (bind _asbp_base_player (cast `/Game/Core/BP_BasePlayer` OtherActor))
  (set `/Game/Core/BP_BasePlayer.MassActor` null _asbp_base_player))

(event `self.ReceiveTick`
  (params (DeltaSeconds :type "Float (single-precision)"))
  (bind _returnvalue_roll (`KismetMathLibrary.BreakRotator` (`self.K2_GetActorRotation`)))
  (`|ExecutionSequence`
    (:`then_0`
      (if (>= (`KismetMathLibrary.Abs` _returnvalue_roll) (`self.AngleThreshold`))
        (set `self.CurrentPushover` (`self.PushoverTolerance`))
        (set `self.HasFallenOff` true)))
    (:`then_1`
      (if (>= (`self.CurrentPushover`) (`self.PushoverTolerance`))
        (`self.CheckFinalPush`)))))

(fn `CheckFinalPush`
  (bind _returnvalue_roll (`KismetMathLibrary.BreakRotator` (`self.K2_GetActorRotation`)))
  (bind _asgm_base_game_mode (cast `/Game/Core/GM_BaseGameMode` (`GameplayStatics.GetGameMode`)))
  (`KismetArrayLibrary.Array_RemoveItem` (`/Game/Core/BP_BaseHouse.MassObjects` (`/Game/Core/GM_BaseGameMode.BaseHouseRef` _asgm_base_game_mode)) (`self.BPC_Mass`))
  (`PrimitiveComponent.SetCollisionEnabled` (`self.Box`) "QueryAndPhysics")
  (`PrimitiveComponent.SetSimulatePhysics` (`self.Box`) true)
  (`PrimitiveComponent.SetEnableGravity` (`self.Box`) true)
  (`PrimitiveComponent.SetConstraintMode` (`self.Box`) "None")
  (`self.K2_DetachFromActor` self "KeepWorld" "KeepWorld" "KeepWorld")
  (`PrimitiveComponent.AddImpulse` (`self.Box`) (select `bool` (`self.HasFallenOff`) :`false` (-1000.0 0.0 0.0) :`true` (* (`self.GetActorRightVector`) (* (`KismetMathLibrary.FClamp` _returnvalue_roll -1.0) 100.0))) "None" true)
  (set `self.HasFallenOff` false)
  (return))

(fn `Pushover`
  (bind _result (`/Engine/EditorBlueprintResources/StandardMacros.IncrementInt` (`self.CurrentPushover`))
    (:`  `
      (if (not (>= _result (`self.PushoverTolerance`)))
        (`self.Shake`)))))

(fn `UserConstructionScript`)