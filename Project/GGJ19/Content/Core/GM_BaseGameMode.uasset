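; Base game mode for a local multiplayer game that shows the main menu, spawns players and game UI, tracks score and caches the house actor.
; StartGame creates a local player per index, spawns a pawn at the PlayerStart tagged with that index and possesses it.
; A pawn-to-index map drives respawning: a destroyed pawn is replaced at its tagged start, repossessed, then destruction events are rebound.
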(event `self.ReceiveBeginPlay`
  (`|ExecutionSequence`
    (:`then_0`
      (bind _returnvalue (`|CreateWidget` "/Game/UI/WBP_MainMenu.WBP_MainMenu_C"))
      (`UserWidget.AddToViewport` _returnvalue 0))
    (:`then_1`
      (bind _outactors (`GameplayStatics.GetAllActorsOfClass` "/Game/Core/BP_BaseHouse.BP_BaseHouse_C"))
      (set `self.BaseHouseRef` (`|GetArrayItem` _outactors)))))

(event `Start Game`
  (`|ExecutionSequence`
    (:`then_0`
      ;[1 1 1] Spawn all players
      (`self.GetStartPoints`)
      (`self.SpawnPlayers`)
      (`self.SpawnUI`))
    (:`then_1`
      (bind _keys (`BlueprintMapLibrary.Map_Keys` (`self.Players`) :!label _label))
      (for _array_element _keys
        (`/Engine/EditorBlueprintResources/StandardMacros.IsValid` _array_element
          (:`Is Valid`
            (add `self.OnDestroyed` _array_element (delegate `OnDestroyed_Event_0`))))))))

(event `Respawn`
  (goto _label))

(event `OnDestroyed_Event_0`
  (params (DestroyedActor :type "Actor Object Reference"))
  (bind _asbp_base_player (cast `/Game/Core/BP_BasePlayer` DestroyedActor))
  (for _array_element (`self.PlayerStarts`)
    (bind _value (`BlueprintMapLibrary.Map_Find` (`self.Players`) _asbp_base_player))
    (if (== (`PlayerStart.PlayerStartTag` _array_element) (`KismetStringLibrary.Conv_StringToName` (`KismetStringLibrary.Conv_IntToString` _value)))
      (bind _returnvalue (`|SpawnActorFromClass` "/Game/Core/BP_BasePlayer.BP_BasePlayer_C" (`self.GetTransform` _array_element) "AdjustIfPossibleButAlwaysSpawn" "OverrideRootScale" null null))
      (bind _returnvalue_2 (`GameplayStatics.GetPlayerController` _value))
      (bind _aspc_base_controller (cast `/Game/Core/PC_BaseController` _returnvalue_2))
      (bind _output_get (set `/Game/Core/PC_BaseController.PlayerRef` _returnvalue _aspc_base_controller))
      (`Controller.Possess` _returnvalue_2 _output_get)
      (`BlueprintMapLibrary.Map_Add` (`self.Players`) _returnvalue _value)
      (`self.Respawn`))))

(fn `GetStartPoints`
  (bind _outactors (`GameplayStatics.GetAllActorsOfClass` "/Script/Engine.PlayerStart"))
  (set `self.PlayerStarts` _outactors))

(fn `SpawnPlayers`
  (locals (currentIndex :type Integer))
  (bind _currentindex (`local.currentIndex`))
  (bind _returnvalue (`GameplayStatics.GetPlayerController` _currentindex))
  (for _index (range (`self.PlayerCount`))
    (set `local.currentIndex` _index)
    (for _array_element (`self.PlayerStarts`)
      (if (== (`PlayerStart.PlayerStartTag` _array_element) (`KismetStringLibrary.Conv_StringToName` (`KismetStringLibrary.Conv_IntToString` (`local.currentIndex`))))
        (`GameplayStatics.CreatePlayer` _currentindex)
        (bind _returnvalue_2 (`|SpawnActorFromClass` "/Game/Core/BP_BasePlayer.BP_BasePlayer_C" (`self.GetTransform` _array_element) "AdjustIfPossibleButAlwaysSpawn" "OverrideRootScale" null null))
        (bind _aspc_base_controller (cast `/Game/Core/PC_BaseController` _returnvalue))
        (bind _output_get (set `/Game/Core/PC_BaseController.PlayerRef` _returnvalue_2 _aspc_base_controller))
        (`Controller.Possess` _returnvalue _output_get)
        (`BlueprintMapLibrary.Map_Add` (`self.Players`) _returnvalue_2 _currentindex)
        (break)))))

(fn `SpawnUI`
  (bind _returnvalue (`|CreateWidget` "/Game/UI/WBP_GameUI.WBP_GameUI_C"))
  (bind _output_get (set `self.GameUI` _returnvalue))
  (`UserWidget.AddToViewport` _output_get 0))

(fn `UpdateScore`
  (params (ScoreToAdd :type "Float (double-precision)"))
  (set `self.Score` (+ ScoreToAdd (`self.Score`)))
  (return))

(fn `UserConstructionScript`)